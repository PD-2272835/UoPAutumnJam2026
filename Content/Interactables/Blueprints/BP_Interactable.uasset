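; BP_Interactable is an interactable item actor whose Item data sets its mesh, trigger radius and prompt name.
; On BeginPlay it fills a widget prompt, building flavour text from the item's stats when none is written, and caches the player.
; Sphere overlaps toggle the prompt and set or clear the player's CurrentInteractable.
; OnInteract only prints a placeholder debug message.
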(event OnComponentBeginOverlap(SC_CollisionTrigger)
  (params (OverlappedComponent :type Primitive%20Component%20Object%20Reference) (OtherActor :type Actor%20Object%20Reference) (OtherComp :type Primitive%20Component%20Object%20Reference) (OtherBodyIndex :type Integer) (bFromSweep :type Boolean) (SweepResult :type Hit%20Result%20Structure%20%28by%20ref%29))
  (if (== OtherActor (Variables|Default|GetPlayerRef))
    (Rendering|SetVisibility (Variables|Default|GetW_Prompt) true false)
    (Variables|/Game/FirstPerson/Blueprints/BP_FirstPersonCharacter.BP_FirstPersonCharacter_C|SetCurrentInteractable (Variables|Default|GetPlayerRef) self)))

(event OnComponentEndOverlap(SC_CollisionTrigger)
  (params (OverlappedComponent :type Primitive%20Component%20Object%20Reference) (OtherActor :type Actor%20Object%20Reference) (OtherComp :type Primitive%20Component%20Object%20Reference) (OtherBodyIndex :type Integer))
  (if (== OtherActor (Variables|Default|GetPlayerRef))
    (if (== self (Variables|/Game/FirstPerson/Blueprints/BP_FirstPersonCharacter.BP_FirstPersonCharacter_C|GetCurrentInteractable (Variables|Default|GetPlayerRef)))
      (Rendering|SetVisibility (Variables|Default|GetW_Prompt) false false)
      (Variables|/Game/FirstPerson/Blueprints/BP_FirstPersonCharacter.BP_FirstPersonCharacter_C|SetCurrentInteractable (Variables|Default|GetPlayerRef) 0))))

(event EventOnInteract
  (Development|PrintString "Interacted with your mother!!!"))

(event EventBeginPlay
  (bind _w_prompt (Variables|Default|GetW_Prompt))
  (bind _item (Variables|Default|GetItem))
  (Rendering|SetVisibility _w_prompt false false)
  (bind _aswbp_prompt (Utilities|Casting|CastToWBP_InteractionPrompt (UserInterface|GetWidget _w_prompt)))
  (Default|SetItemName _aswbp_prompt (Utilities|Text|ToText(String) (.name _item)))
  (|FlavourTextSetting (.stat _item)
    (:CompletedPin
      (Default|SetFlavourText _aswbp_prompt (Utilities|Text|ToText(String) (Variables|Default|GetFlavourText)))
      ;[0.15 0.15 0.15 0.5] no point in casting all the friggin time, also it's single player
      (bind _asbp_first_person_character (Utilities|Casting|CastToBP_FirstPersonCharacter (Game|GetPlayerCharacter 0)))
      (Variables|Default|SetPlayerRef _asbp_first_person_character))))

(fn ConstructionScript
  (bind _item (Variables|Default|GetItem))
  (Components|Sphere|SetSphereRadius (Variables|Default|GetSC_CollisionTrigger) (.interactdistance _item) true)
  (Components|StaticMesh|SetStaticMesh (Variables|Default|GetSM_Model) (.mesh _item)))